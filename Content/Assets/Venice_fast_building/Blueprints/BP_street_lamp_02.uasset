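; Street lamp prop Blueprint with a mesh and spot light that can be switched on or off per instance.
; The construction script toggles spot light visibility from the Light flag and applies the exposed Color and Intensity.
; It creates a dynamic material instance on the mesh and sets its emissive power to match the on/off state.
; The event graph holds no active logic.
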(fn `UserConstructionScript`
  (bind _light (`self.light`))
  (`SceneComponent.SetVisibility` (`self.SpotLight`) _light false)
  (bind _returnvalue (`PrimitiveComponent.CreateDynamicMaterialInstance` (`self.mesh`) 0 "/Game/Assets/Venice_fast_building/Materials/MI_street_lamp_02.MI_street_lamp_02" "None"))
  (if _light
    (`MaterialInstanceDynamic.SetScalarParameterValue` _returnvalue "emissive power" 20.0)
    (else
      (`MaterialInstanceDynamic.SetScalarParameterValue` _returnvalue "emissive power" 0.0)))
  (`LightComponent.SetLightColor` (`self.SpotLight`) (`self.color`) true)
  (`LightComponent.SetIntensity` (`self.SpotLight`) (`self.intensity`)))